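; Player controller for a top-down game that drives movement of the possessed TD_Character through Enhanced Input.
; BeginPlay adds the IMC_TopDown mapping context and casts the pawn to TD_Character without using the result.
; While IA_Move triggers, it casts the controlled pawn again and feeds the 2D input to AddMovementInput as a world-space XY direction, independent of camera or control rotation.
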(event Input|EnhancedActionEvents|EnhancedInputActionIA_Move
  (params (ActionValue :type Vector%202D%20Structure) (ElapsedSeconds :type Float%20%28double-precision%29) (TriggeredSeconds :type Float%20%28double-precision%29) (InputAction :type Input%20Action%20Object%20Reference :default "/Game/Blueprints/Input/IA_Move.IA_Move"))
  (bind _returnvalue (Input|EnhancedActionValues|GetIA_Move))
  (bind (_x _y) (Math|Vector2D|BreakVector2D _returnvalue))
  (:Triggered
    (bind _astd_character (Utilities|Casting|CastToTD_Character (Pawn|GetControlledPawn)))
    (Pawn|Input|AddMovementInput _astd_character (Math|Conversions|ToVector(Vector2D) (Math|Vector2D|MakeVector2D _x _y)) 1.0 false)))

(event EventBeginPlay
  (Input|AddMappingContext (PlayerController|LocalPlayerSubsystems|GetEnhancedInputLocalPlayerSubsystem) "/Game/Blueprints/Input/IMC_TopDown.IMC_TopDown" 0 "(bIgnoreAllPressedKeysUntilRelease=True,bForceImmediately=False,bNotifyUserSettings=False)")
  (Utilities|Casting|CastToTD_Character (Pawn|GetControlledPawn)))

(fn ConstructionScript)